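; BP_Enemy is an enemy actor whose ship mesh takes one of four coin materials based on EnemyId, named for none, bullet speed, big bullet and move speed.
; BeginPlay applies that material and a random starting yaw from a random stream, and Tick keeps it spinning by a fixed, frame-dependent yaw step.
; SpawnExplosion spawns an explosion emitter at the actor's location, tinted with its primary and secondary colors.
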(event `self.ReceiveBeginPlay`
  (bind _shipsm (`self.ShipSM`))
  (`self.K2_AddActorLocalRotation` (`KismetMathLibrary.MakeRotator` 0.0 0.0 (`KismetMathLibrary.Conv_IntToDouble` (`KismetMathLibrary.RandomIntegerInRangeFromStream` 45 180 (`self.RandomStream`)))))
  (switch `int` (`self.EnemyId`)
    (:`0`
      (`PrimitiveComponent.SetMaterial` _shipsm 0 "/Game/SpaceshipBattle/Materials/Coin/M_Coin_None.M_Coin_None"))
    (:`1`
      (`PrimitiveComponent.SetMaterial` _shipsm 0 "/Game/SpaceshipBattle/Materials/Coin/M_Coint_Speed_Bull.M_Coint_Speed_Bull"))
    (:`2`
      (`PrimitiveComponent.SetMaterial` _shipsm 0 "/Game/SpaceshipBattle/Materials/Coin/M_Coint_Big_Bullt.M_Coint_Big_Bullt"))
    (:`3`
      (`PrimitiveComponent.SetMaterial` _shipsm 0 "/Game/SpaceshipBattle/Materials/Coin/M_Coin_Speed_Move.M_Coin_Speed_Move"))))

(event `self.ReceiveTick`
  (params (DeltaSeconds :type "Float (single-precision)"))
  (`self.K2_AddActorLocalRotation` (struct :`Yaw` 0.3)))

(event `self.SetColor`)

(event `self.SpawnExplosion`
  (bind _returnvalue (`GameplayStatics.SpawnEmitterAtLocation` "/Game/ParticleSystem/PS_Explosion.PS_Explosion" (`self.K2_GetActorLocation`)))
  (`ParticleSystemComponent.SetColorParameter` _returnvalue "PrimaryColor" (`self.PrimaryColor`))
  (`ParticleSystemComponent.SetColorParameter` _returnvalue "SecondryColor" (`self.SecondryColor`)))

(fn `UserConstructionScript`)