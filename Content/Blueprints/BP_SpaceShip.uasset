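; BP_SpaceShip is the player's input-side spaceship, which creates the score HUD and caches the BP_NetworkPlay actor on BeginPlay.
; The turn axes combine into an integer yaw angle, and any nonzero result also sets firing, so a yaw truncating to zero never fires.
; MoveRight sends the truncated move axes, angle and fire flag through SendInputPackage on every axis update, with no local movement in this Blueprint.
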(event `self.ReceiveTick`
  (params (DeltaSeconds :type "Float (single-precision)")))

(event `self.ReceiveBeginPlay`
  (bind _returnvalue (`|CreateWidget` "/Game/Blueprints/UI/WBP_Score.WBP_Score_C"))
  (`UserWidget.AddToViewport` _returnvalue 0)
  (bind _returnvalue_2 (`GameplayStatics.GetActorOfClass` "/Game/Blueprints/Network/BP_NetworkPlay.BP_NetworkPlay_C"))
  (set `self.Network` _returnvalue_2))

(event `InputAxis|TurnUp`
  (params (AxisValue :type "Float (single-precision)"))
  (set `self.TempUp` AxisValue))

(event `InputAxis|TurnRight`
  (params (AxisValue :type "Float (single-precision)"))
  (bind _returnvalue (`KismetMathLibrary.FTrunc` (.yaw (`KismetMathLibrary.MakeRotFromX` (`KismetMathLibrary.MakeVector` (`self.TempUp`) AxisValue)))))
  (if (!= _returnvalue 0)
    (set `self.PressFire` true)
    (set `self.Angle` _returnvalue)
    (else
      (set `self.PressFire` false))))

(event `InputAxis|MoveUp`
  (params (AxisValue :type "Float (single-precision)"))
  (set `self.Up` (`KismetMathLibrary.FTrunc` AxisValue)))

(event `InputAxis|MoveRight`
  (params (AxisValue :type "Float (single-precision)"))
  (`NetworkPlay.SendInputPackage` (`self.Network`) (`self.Up`) (`KismetMathLibrary.FTrunc` AxisValue) (`self.Angle`) (`self.PressFire`)))

(fn `UserConstructionScript`)